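; Area actor, named for frost, that applies a gameplay effect to pawns entering its EffectArea component.
; On BeginPlay it asynchronously loads the configured effect class and caches it once the cast to BP_GameplayEffect succeeds.
; Overlaps from components tagged PawnCapsule apply that class at level 1 through the other actor's BP_AdvancedAbilitySystemComponent, passing its location and this area as causer.
; Nothing in this graph removes the effect on exit.
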(event OnComponentBeginOverlap(EffectArea)
  (params (OverlappedComponent :type Primitive%20Component%20Object%20Reference) (OtherActor :type Actor%20Object%20Reference) (OtherComp :type Primitive%20Component%20Object%20Reference) (OtherBodyIndex :type Integer) (bFromSweep :type Boolean) (SweepResult :type Hit%20Result%20Structure%20%28by%20ref%29))
  (if (Components|ComponentHasTag OtherComp "PawnCapsule")
    (Default|ApplyGameplayEffectbyClass (Actor|GetComponentbyClass OtherActor "/Game/AdvancedARPGCombat/AdvancedCombatFramework/AbilitySystem/BP_AdvancedAbilitySystemComponent.BP_AdvancedAbilitySystemComponent_C") (Variables|Default|GetGameplayEffectClassRef) 1 (Utilities|Struct|MakeF_EffectData "(GameplayTags=)" (Transformation|GetActorLocation OtherActor) 0 self 0))))

(event EventBeginPlay
  (bind _class (Utilities|AsyncLoadClassAsset (Variables|GameplayEffect|GetGameplayEffectClass))
    (:Completed
      (bind _asbp_gameplay_effect (Utilities|Casting|CastToBP_GameplayEffectClass _class))
      (Variables|Default|SetGameplayEffectClassRef _asbp_gameplay_effect))))

(event Collision|EventActorBeginOverlap
  (params (OtherActor :type Actor%20Object%20Reference)))

(event EventTick
  (params (DeltaSeconds :type Float%20%28single-precision%29)))

(fn ConstructionScript)