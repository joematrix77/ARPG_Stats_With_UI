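; BP_LightningCue is a gameplay cue that shows a lightning status effect with particles and a HUD indicator.
; On execute it attaches a scaled-down emitter at the Pelvis and adds a lightning widget to player 0's status effect list.
; The list's container is cached on the game instance and recreated if invalid or off-screen.
; On remove it destroys only the particle component, leaving the widget untouched.
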(event EventOnExecute
  (params (GameplayCueData :type F%20Gameplay%20Cue%20Data%20Structure%20%28by%20ref%29))
  (bind _returnvalue (Game|GetPlayerController 0))
  (bind _returnvalue_2 (Effects|SpawnEmitterAttached 0 0 "Pelvis" "0, 0, 0" "0, 0, 0" "0.800000,0.800000,0.800000"))
  (Variables|Default|SetLightningParticleComponent _returnvalue_2)
  (bind _asbp_advanced_game_instance (Utilities|Casting|CastToBP_AdvancedGameInstance (Game|GetGameInstance)))
  (if (and (Utilities|IsValid (Variables|/Game/AdvancedARPGCombat/MeleeCombatSystem/Blueprints/BP_AdvancedGameInstance.BP_AdvancedGameInstance_C|GetStatusEffectContainer _asbp_advanced_game_instance)) (UserInterface|Viewport|IsinViewport (Variables|/Game/AdvancedARPGCombat/MeleeCombatSystem/Blueprints/BP_AdvancedGameInstance.BP_AdvancedGameInstance_C|GetStatusEffectContainer _asbp_advanced_game_instance)))
    _
    (else
      (bind _returnvalue_3 (UserInterface|CreateWidget "/ARPG_Stats/Widget/StatusEffects/WBP_StatusEffectContainer.WBP_StatusEffectContainer_C" _returnvalue))
      (bind _output_get (Variables|/Game/AdvancedARPGCombat/MeleeCombatSystem/Blueprints/BP_AdvancedGameInstance.BP_AdvancedGameInstance_C|SetStatusEffectContainer _asbp_advanced_game_instance _returnvalue_3))
      (UserInterface|Viewport|AddtoViewport _output_get 0)))
  (bind _returnvalue_4 (UserInterface|CreateWidget "/ARPG_Stats/Widget/StatusEffects/WB_LightningEffect.WB_LightningEffect_C" _returnvalue))
  (Class|VerticalBox|AddChildtoVerticalBox (Variables|/ARPG_Stats/Widget/StatusEffects/WBP_StatusEffectContainer.WBP_StatusEffectContainer_C|GetEffectList (Variables|/Game/AdvancedARPGCombat/MeleeCombatSystem/Blueprints/BP_AdvancedGameInstance.BP_AdvancedGameInstance_C|GetStatusEffectContainer _asbp_advanced_game_instance)) _returnvalue_4))

(event EventOnRemove
  (bind _lightningparticlecomponent (Variables|Default|GetLightningParticleComponent)
    (:then
      (Components|DestroyComponent _lightningparticlecomponent))
    (:else)))

(fn ConstructionScript
  (|CallParentFunction))