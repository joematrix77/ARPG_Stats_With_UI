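; Gameplay cue for the poisoned status, showing it on the affected character and on the HUD.
; On execute it attaches a scaled-down poison emitter to the mesh's pelvis and adds a poison widget to the status effect container.
; That container is shared through the game instance and created on demand if missing or off-screen.
; On remove it destroys only the particle component, leaving the widget to other logic.
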(event EventOnExecute
  (params (GameplayCueData :type F%20Gameplay%20Cue%20Data%20Structure%20%28by%20ref%29))
  (bind _returnvalue (Game|GetPlayerController 0))
  (bind _returnvalue_2 (Effects|SpawnEmitterAttached (Variables|Default|GetPoisoned%20Emitter%20Template) (Variables|/Script/Engine.Character|GetMesh (.AsCharacter (Utilities|Casting|CastToCharacter (Components|GetOwner)))) "Pelvis" "0, 0, 0" "0, 0, 0" "0.800000,0.800000,0.800000"))
  (Variables|Default|SetPoisonedParticleComponent _returnvalue_2)
  (bind _asbp_advanced_game_instance (Utilities|Casting|CastToBP_AdvancedGameInstance (Game|GetGameInstance)))
  (bind _output_get (Variables|Default|SetEffect%20Container (Variables|/Game/AdvancedARPGCombat/MeleeCombatSystem/Blueprints/BP_AdvancedGameInstance.BP_AdvancedGameInstance_C|GetEffectContainer _asbp_advanced_game_instance)))
  (if (and (Utilities|IsValid _output_get) (UserInterface|Viewport|IsinViewport _output_get))
    _
    (else
      (bind _returnvalue_3 (UserInterface|CreateWidget "/ARPG_Stats/Widget/StatusEffects/WBP_StatusEffectContainer.WBP_StatusEffectContainer_C" _returnvalue))
      (bind _output_get_2 (Variables|/Game/AdvancedARPGCombat/MeleeCombatSystem/Blueprints/BP_AdvancedGameInstance.BP_AdvancedGameInstance_C|SetEffectContainer _asbp_advanced_game_instance _returnvalue_3))
      (UserInterface|Viewport|AddtoViewport _output_get_2 0)))
  (bind _returnvalue_4 (UserInterface|CreateWidget "/ARPG_Stats/Widget/StatusEffects/WB_PoisonEffect.WB_PoisonEffect_C" _returnvalue))
  (Class|VerticalBox|AddChildtoVerticalBox (Variables|/ARPG_Stats/Widget/StatusEffects/WBP_StatusEffectContainer.WBP_StatusEffectContainer_C|GetEffectList (Variables|/Game/AdvancedARPGCombat/MeleeCombatSystem/Blueprints/BP_AdvancedGameInstance.BP_AdvancedGameInstance_C|GetEffectContainer _asbp_advanced_game_instance)) _returnvalue_4))

(event EventOnRemove
  (bind _poisonedparticlecomponent (Variables|Default|GetPoisonedParticleComponent)
    (:then
      (Components|DestroyComponent _poisonedparticlecomponent))
    (:else)))

(fn ConstructionScript
  (|CallParentFunction))