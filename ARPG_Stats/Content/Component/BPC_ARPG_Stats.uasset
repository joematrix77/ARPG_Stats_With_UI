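; Actor component that levels up the player's Health, Mana and Stamina stats, currently triggered by numpad debug keys.
; BeginPlay async-loads the player info asset, caches the owner's BP_AttributesComponent and calls a UI update.
; Each upgrade increments a clamped level, reads its value from CT_LevelCurves, modifies the attribute, sets the clamped result on its Max tag and broadcasts it.
; The tag-based LevelUp handles only Health and its EventGraph call is disconnected.
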(event EventBeginPlay
  (|CallParentFunction)
  (bind _object (Utilities|AsyncLoadAsset (Variables|Initialization|GetPlayerInfo))
    (:Completed
      (bind _asbp_player_info (Utilities|Casting|CastToBP_PlayerInfo _object))
      (bind _output_get (Variables|Initialization|SetPlayerInfoRef _asbp_player_info))
      (Utilities|IsValid _output_get
        (:Is%20Valid
          (Variables|Default|SetAttributesComponent (Actor|GetComponentbyClass (Components|GetOwner) "/Game/AdvancedARPGCombat/AdvancedCombatFramework/AttributesSystem/BP_AttributesComponent.BP_AttributesComponent_C"))
          (Default|CallUpdateUI))
        (:Is%20Not%20Valid
          (CallFunction|DisplayDeveloperWarning "Player info is Not Valid"))))))

(event EventTick
  (params (DeltaSeconds :type Float%20%28single-precision%29)))

(event Input|KeyboardEvents|DebugKeyNumPadOne
  (params (Key :type Key%20Structure :default "None") (ActionValue :type Input%20Action%20Value%20Structure))
  (:Pressed
    (Setters|SetHealthStat)))

(event Input|KeyboardEvents|DebugKeyNumPadTwo
  (params (Key :type Key%20Structure :default "None") (ActionValue :type Input%20Action%20Value%20Structure))
  (:Pressed
    (Setters|SetManaStat)))

(event Input|KeyboardEvents|DebugKeyNumPadThree
  (params (Key :type Key%20Structure :default "None") (ActionValue :type Input%20Action%20Value%20Structure))
  (:Pressed
    (Setters|SetStaminaStat)))

(fn SetHealthStat
  (bind _attributescomponent (Variables|Default|GetAttributesComponent))
  (bind _returnvalue (CallFunction|SetHealthAttribute))
  (Development|PrintString (Utilities|String|Append "Current Health Upgraded By - " (Utilities|String|ToString(Float) _returnvalue) " Points") true true "(R=0.000000,G=0.660000,B=1.000000,A=1.000000)" 1e+01)
  (bind _modified_attribute_value (Default|ModifyAttribute _attributescomponent "(TagName=\"Attribute.Health\")" "NewEnumerator0" "NewEnumerator0" _returnvalue))
  (Default|SetCurrentAttributeValue _attributescomponent "(TagName=\"Attribute.HealthMax\")" (Math|Float|Clamp(Float) _modified_attribute_value 1.0 5e+02))
  (Default|CallOnCurrentAttributeValueUpdated "(TagName=\"Attribute.HealthMax\")" (Math|Float|Clamp(Float) _modified_attribute_value 1.0 5e+02)))

(fn GetPlayerInfo
  (return (Variables|Initialization|GetPlayerInfoRef)))

(fn SetHealthAttribute
  (bind _result (Math|Integer|IncrementInt (Variables|Default|GetLevelHealth))
    (:%20%20
      (bind _structout (Utilities|Struct|SetmembersinS_LevelProgression (Variables|Default|GetPlayerLevel) (Math|Integer|Clamp(Integer) _result 1 158)))
      (bind _output_get (Variables|Default|SetLevelHealth (Utilities|Struct|BreakS_LevelProgression _structout)))
      (Development|PrintString (Utilities|String|Append "Current Health Level Is -  
" (Utilities|String|ToString(Integer) (Math|Integer|Clamp(Integer) _result 1 158))))
      (bind _outxy (DataTable|EvaluateCurveTableRow "/ARPG_Stats/DataTables/CT_LevelCurves.CT_LevelCurves" "Attribute.Health" (Math|Conversions|ToFloat(Integer) _output_get) "Get Health Level Value")
        (:RowFound
          (bind _output_get_2 (LocalVariables|SetL_AttributeHealth _outxy))
          (bind _structout_2 (Utilities|Struct|SetmembersinS_StatProgression (Variables|Default|GetPlayerStats) _output_get_2))
          (return (Utilities|Struct|BreakS_StatProgression _structout_2) (Variables|Default|GetLevelHealth)))))))

(fn SetManaAttribute
  (bind _result (Math|Integer|IncrementInt (Variables|Default|GetLevelMana))
    (:%20%20
      (bind _structout (Utilities|Struct|SetmembersinS_LevelProgression (Variables|Default|GetPlayerLevel) (Math|Integer|Clamp(Integer) _result 1 166)))
      (bind _output_get (Variables|Default|SetLevelMana (Utilities|Struct|BreakS_LevelProgression _structout)))
      (Development|PrintString (Utilities|String|Append "Current Mana Level Is -  
" (Utilities|String|ToString(Integer) _output_get)))
      (bind _outxy (DataTable|EvaluateCurveTableRow "/ARPG_Stats/DataTables/CT_LevelCurves.CT_LevelCurves" "Attribute.Mana" (Math|Conversions|ToFloat(Integer) _output_get) "Get Mana Level Value")
        (:RowFound
          (bind _output_get_2 (LocalVariables|SetL_AttributeMana _outxy))
          (bind _structout_2 (Utilities|Struct|SetmembersinS_StatProgression (Variables|Default|GetPlayerStats) _output_get_2))
          (return (Utilities|Struct|BreakS_StatProgression _structout_2) (Variables|Default|GetLevelMana)))))))

(fn SetManaStat
  (bind _attributescomponent (Variables|Default|GetAttributesComponent))
  (bind _returnvalue (CallFunction|SetManaAttribute))
  (Development|PrintString (Utilities|String|Append "Current Mana Upgraded By - " (Utilities|String|ToString(Float) _returnvalue) " Points") true true "(R=0.000000,G=0.660000,B=1.000000,A=1.000000)" 1e+01)
  (bind _modified_attribute_value (Default|ModifyAttribute _attributescomponent "(TagName=\"Attribute.Mana\")" "NewEnumerator0" "NewEnumerator0" _returnvalue))
  (Default|SetCurrentAttributeValue _attributescomponent "(TagName=\"Attribute.ManaMax\")" (Math|Float|Clamp(Float) _modified_attribute_value 1.0 511.72))
  (Default|CallOnCurrentAttributeValueUpdated "(TagName=\"Attribute.ManaMax\")" (Math|Float|Clamp(Float) _modified_attribute_value 1.0 511.72)))

(fn SetStaminaStat
  (bind _attributescomponent (Variables|Default|GetAttributesComponent))
  (bind _returnvalue (CallFunction|SetStaminaAttribute))
  (Development|PrintString (Utilities|String|Append "Current Stamina Upgraded By - " (Utilities|String|ToString(Float) _returnvalue) " Points") true true "(R=0.000000,G=0.660000,B=1.000000,A=1.000000)" 1e+01)
  (bind _modified_attribute_value (Default|ModifyAttribute _attributescomponent "(TagName=\"Attribute.Stamina\")" "NewEnumerator0" "NewEnumerator0" _returnvalue))
  (Default|SetCurrentAttributeValue _attributescomponent "(TagName=\"Attribute.StaminaMax\")" (Math|Float|Clamp(Float) _modified_attribute_value 1.0 5.5e+02))
  (Default|CallOnCurrentAttributeValueUpdated "(TagName=\"Attribute.StaminaMax\")" (Math|Float|Clamp(Float) _modified_attribute_value 1.0 5.5e+02)))

(fn SetStaminaAttribute
  (bind _result (Math|Integer|IncrementInt (Variables|Default|GetLevelStamina))
    (:%20%20
      (bind _structout (Utilities|Struct|SetmembersinS_LevelProgression (Variables|Default|GetPlayerLevel) (Math|Integer|Clamp(Integer) _result 1 172)))
      (bind _output_get (Variables|Default|SetLevelStamina (Utilities|Struct|BreakS_LevelProgression _structout)))
      (Development|PrintString (Utilities|String|Append "Current Stamina Level Is -  
" (Utilities|String|ToString(Integer) _output_get)))
      (bind _outxy (DataTable|EvaluateCurveTableRow "/ARPG_Stats/DataTables/CT_LevelCurves.CT_LevelCurves" "Attribute.Stamina" (Math|Conversions|ToFloat(Integer) _output_get) "Get Mana Level Value")
        (:RowFound
          (bind _output_get_2 (LocalVariables|SetL_AttributeStamina _outxy))
          (bind _structout_2 (Utilities|Struct|SetmembersinS_StatProgression (Variables|Default|GetPlayerStats) _output_get_2))
          (return (Utilities|Struct|BreakS_StatProgression _structout_2) (Variables|Default|GetLevelStamina)))))))

(fn LevelUp
  (params (AttributeTag :type Gameplay%20Tag%20Structure))
  (|SwitchGameplayTag AttributeTag
    (:Attribute.Health
      (Setters|SetHealthStat)
      (Variables|Default|SetLevel 0))))