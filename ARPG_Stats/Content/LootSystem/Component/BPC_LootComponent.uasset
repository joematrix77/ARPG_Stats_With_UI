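; BPC_LootComponent is an actor component that rolls loot from a supplied LootInfo list and drops it as a pickup at its owner's location.
; SpawnLoot rolls each entry's quantity against its drop probability and gathers the successful items into one list.
; A random rarity roll bounded by the player's LevelLuck stat gates updates to the best rarity.
; That rarity selects the pickup actor class, which spawns holding all looted items.
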(event Custom|WaitToNextTick
  (Utilities|FlowControl|DelayUntilNextTick))

(event EventBeginPlay)

(fn Initialize
  (params (LootInfo :type Array%20of%20S%20Loot%20Structures))
  (Variables|Default|SetLootInfo LootInfo))

(fn SpawnLoot
  (LocalVariables|SetL_BestRarity "NewEnumerator0")
  (Utilities|FlowControl|Sequence
    (:then_0
      (for _array_element (Variables|Default|GetLootInfo)
        (LocalVariables|SetL_LootableItem (.LootableItem (Utilities|Struct|BreakS_Loot _array_element)))
        (bind _lootedquantity (CallFunction|RandomizeLootedQuantity (.LootProbability (Utilities|Struct|BreakS_Loot _array_element)) (.MaxQuantityLootable (Utilities|Struct|BreakS_Loot _array_element))))
        (if (> _lootedquantity 0)
          (Utilities|Array|Add (LocalVariables|GetL_LootedItems) (Utilities|Struct|MakeF_ItemSlot (LocalVariables|GetL_LootableItem) _lootedquantity 0 false "00000000000000000000000000000000"))
          (bind _raritydrop (CallFunction|RandomLuckDrop))
          (if (Math|Integer|InRange(Integer) (Math|Conversions|ToInteger(Byte) _raritydrop) (Math|Conversions|ToInteger(Byte) (LocalVariables|GetL_BestRarity)) (Math|Conversions|ToInteger(Byte) _raritydrop))
            (LocalVariables|SetL_BestRarity (Variables|/Game/AdvancedARPGCombat/AdvancedCombatFramework/InventorySystem/Items/BP_ItemBase.BP_ItemBase_C|GetItemRarity (LocalVariables|GetL_LootableItem)))))))
    (:then_1
      (if (> (Utilities|Array|Length (LocalVariables|GetL_LootedItems)) 0)
        ;[0.15 0.15 0.15 0.5] Can Be Removed Using for Testing when Killing Multiple Enemies at once drops fall out of sync and will drop items out of your stat level
        (CallFunction|WaittoNextTick)
        (Game|SpawnActorfromClass (.Value (Utilities|Map|Find (Variables|Default|GetPickupActors) (.Value (Utilities|Map|Find (LocalVariables|GetL_IndexRarity) (Math|Conversions|ToInteger(Byte) (LocalVariables|GetL_BestRarity)))))) (Math|Transform|MakeTransform (Transformation|GetActorLocation (Components|GetOwner)) "0, 0, 0" "1.000000,1.000000,1.000000") "Undefined" "MultiplyWithRoot" 0 (LocalVariables|GetL_LootedItems) true 0)))))

(fn RandomizeLootedQuantity
  (params (LootProbability :type Float%20%28double-precision%29) (MaxLootQuantity :type Integer))
  (if (< LootProbability 1.0)
    (for _index (range 1 MaxLootQuantity)
      (if (<= (Math|Random|RandomFloat) LootProbability)
        (Math|Integer|IncrementInt (LocalVariables|GetL_LootedQuantity))))
    (return (LocalVariables|GetL_LootedQuantity))
    (else
      (return MaxLootQuantity))))

(fn RandomLuckDrop
  (for _array_element (Variables|Default|GetLootInfo)
    (LocalVariables|SetL_LootableItem (Utilities|Struct|BreakS_Loot _array_element))
    (LocalVariables|SetL_LevelLuck (Variables|/ARPG_Stats/Component/BPC_StatsComponent.BPC_StatsComponent_C|GetLevelLuck (Actor|GetComponentbyClass (Game|GetPlayerCharacter 0) "/ARPG_Stats/Component/BPC_StatsComponent.BPC_StatsComponent_C")))
    (if (.ReturnValue (Utilities|Map|Find (LocalVariables|GetL_IndexRarity) (Math|Random|RandomInteger (LocalVariables|GetL_LevelLuck))))
      (bind _output_get (Variables|/Game/AdvancedARPGCombat/AdvancedCombatFramework/InventorySystem/Items/BP_ItemBase.BP_ItemBase_C|SetItemRarity (LocalVariables|GetL_LootableItem) (.Value (Utilities|Map|Find (LocalVariables|GetL_IndexRarity) (Math|Random|RandomInteger (LocalVariables|GetL_LevelLuck))))))
      (return _output_get)
      (else
        (return "NewEnumerator0")))))