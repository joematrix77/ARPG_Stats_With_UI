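; Damage execution for bleed, which lowers the target's BleedResist attribute by the computed damage.
; Execute builds damage from the causer's attack attribute through bonus, critical and resistance steps, using both actors' attribute components.
; DealDamage compares the ModifyAttribute result to BleedResistMax and, if at or below it, applies GE_Bleed through the target's ability system component, crediting the causer.
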(event EventExecute
  (params (EventData :type F%20Gameplay%20Event%20Data%20Structure%20%28by%20ref%29))
  (Variables|Default|SetEventData EventData)
  (CallFunction|SetDamage 0.0)
  (bind _asge_damage_base (Utilities|Casting|CastToGE_DamageBase (CallFunction|GetGameplayEffect))
    (:then
      (Variables|Default|SetDamageGameplayEffect _asge_damage_base))
    (:CastFailed
      _))
  (Variables|Default|SetCauserAttributesComponent (Actor|GetComponentbyClass (Variables|/Script/Engine.Actor|GetInstigator (CallFunction|GetCauser)) "/Game/AdvancedARPGCombat/AdvancedCombatFramework/AttributesSystem/BP_AttributesComponent.BP_AttributesComponent_C"))
  (Variables|Default|SetTargetAttributesComponent (Actor|GetComponentbyClass (CallFunction|GetTarget) "/Game/AdvancedARPGCombat/AdvancedCombatFramework/AttributesSystem/BP_AttributesComponent.BP_AttributesComponent_C"))
  (if (CallFunction|CanDamagebeApplied?)
    (CallFunction|PreCalculationBonus)
    (CallFunction|SetDamage (+ (CallFunction|GetDamage) (Default|GetCurrentAttributeValue (Variables|Default|GetCauserAttributesComponent) (Variables|Default|GetAttackAttributeTag))))
    (CallFunction|CriticalDamage)
    (CallFunction|PostCalculationBonus)
    (bind _output_damage (CallFunction|DamageResist (CallFunction|GetDamage)))
    (CallFunction|SetDamage _output_damage)
    (CallFunction|DealDamage)
    (Variables|Default|SetDamageGameplayEffect 0)))

(fn DealDamage
  (bind _causer (CallFunction|GetCauser))
  (bind _target (CallFunction|GetTarget))
  (bind _returnvalue (Actor|GetComponentbyClass _target "/Game/AdvancedARPGCombat/AdvancedCombatFramework/AbilitySystem/BP_AdvancedAbilitySystemComponent.BP_AdvancedAbilitySystemComponent_C"))
  (Utilities|IsValid (Variables|Default|GetTargetAttributesComponent)
    (:Is%20Valid
      (bind _modified_attribute_value (Default|ModifyAttribute (Variables|Default|GetTargetAttributesComponent) "(TagName=\"Attribute.BleedResist\")" "NewEnumerator1" "NewEnumerator0" (* (CallFunction|GetDamage) -1.0)))
      (if (<= _modified_attribute_value (Default|GetCurrentAttributeValue (Variables|Default|GetTargetAttributesComponent) "(TagName=\"Attribute.BleedResistMax\")"))
        (Utilities|IsValid _returnvalue
          (:Is%20Valid
            (Default|ApplyGameplayEffectbyClass _returnvalue "/ARPG_Stats/Status/GameplayEffect/GE_Bleed.GE_Bleed_C" 1 (Utilities|Struct|MakeF_EffectData (Variables|Default|GetSourceTags) "0.000000,0.000000,0.000000" _causer _causer 0))))))))